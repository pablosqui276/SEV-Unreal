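; BP_Player is the player character, with Enhanced Input movement, jumping and a sword-sound attack that fires a projectile.
; BeginPlay adds the mapping context, and both move inputs push along fixed world axes, then snap control rotation to face the velocity.
; Attack is gated by a DoOnce that resets after timed delays, toggling an animation flag and spawning Player_Projectile at the actor's transform mid-swing.
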(event Custom|RotateInVelocity
  (Pawn|SetControlRotation (Game|GetPlayerController 0) (Math|Conversions|RotationFromXVector (Transformation|GetVelocity))))

(event Custom|Attack
  (Utilities|FlowControl|DoOnce false :!label _label
    (:Completed
      (Variables|Default|SetAnimIsAttacking true)
      (Audio|PlaySound2D "/Game/Sounds/sword.sword" 1.0 1.0 0.0 0 0)
      (Utilities|FlowControl|Delay 0.2)
      (Game|SpawnActorfromClass "/Game/Player_Projectile.Player_Projectile_C" (Transformation|GetActorTransform) "Undefined" "MultiplyWithRoot" 0 0)
      (Utilities|FlowControl|Delay 0.8)
      (Variables|Default|SetAnimIsAttacking false)
      (goto _label Reset))))

(event Input|EnhancedActionEvents|EnhancedInputActionIA_MoveInX
  (params (ActionValue :type Float%20%28double-precision%29) (ElapsedSeconds :type Float%20%28double-precision%29) (TriggeredSeconds :type Float%20%28double-precision%29) (InputAction :type Input%20Action%20Object%20Reference :default "/Game/Player/IA_MoveInX.IA_MoveInX"))
  ;[0.15 0.15 0.15 0.5] Movement
  (Pawn|Input|AddMovementInput "-1.000000,0.000000,0.000000" ActionValue false)
  (CallFunction|RotateinVelocity))

(event Input|EnhancedActionEvents|EnhancedInputActionIA_MoveInY
  (params (ActionValue :type Float%20%28double-precision%29) (ElapsedSeconds :type Float%20%28double-precision%29) (TriggeredSeconds :type Float%20%28double-precision%29) (InputAction :type Input%20Action%20Object%20Reference :default "/Game/Player/IA_MoveInY.IA_MoveInY"))
  ;[0.15 0.15 0.15 0.5] Movement
  (Pawn|Input|AddMovementInput "0.000000,1.000000,0.000000" ActionValue false)
  (CallFunction|RotateinVelocity))

(event Input|EnhancedActionEvents|EnhancedInputActionIA_Attack
  (params (ActionValue :type Boolean) (ElapsedSeconds :type Float%20%28double-precision%29) (TriggeredSeconds :type Float%20%28double-precision%29) (InputAction :type Input%20Action%20Object%20Reference :default "/Game/Player/IA_Attack.IA_Attack"))
  (Development|PrintString "Attack")
  (CallFunction|Attack))

(event Input|EnhancedActionEvents|EnhancedInputActionIA_Jump
  (params (ActionValue :type Boolean) (ElapsedSeconds :type Float%20%28double-precision%29) (TriggeredSeconds :type Float%20%28double-precision%29) (InputAction :type Input%20Action%20Object%20Reference :default "/Game/Player/IA_Jump.IA_Jump"))
  ;[0.15 0.15 0.15 0.5] Saltar
  (:Triggered
    (Character|Jump))
  (:Completed
    (Character|StopJumping)))

(event EventBeginPlay
  ;[0.15 0.15 0.15 0.5] Associate mapping contenxt
  (Input|AddMappingContext (PlayerController|LocalPlayerSubsystems|GetEnhancedInputLocalPlayerSubsystem (Game|GetPlayerController 0)) "/Game/Player/PlayerMapping.PlayerMapping" 0 "(bIgnoreAllPressedKeysUntilRelease=True,bForceImmediately=False,bNotifyUserSettings=False)"))

(event Collision|EventActorBeginOverlap
  (params (OtherActor :type Actor%20Object%20Reference)))

(event EventTick
  (params (DeltaSeconds :type Float%20%28single-precision%29)))

(fn ConstructionScript)