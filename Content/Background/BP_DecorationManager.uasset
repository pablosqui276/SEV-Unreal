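; BP_DecorationManager scatters random background houses across the map when play begins.
; For each house, it picks a random point inside the MapSIze box and spawns a BP_GenericHouse with a random mesh from HouseMeshed.
; A 30-unit distance check runs against OccupiedLocations, but its result never gates spawning, so every candidate is recorded and houses can overlap.
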(event EventBeginPlay
  ;[0.15 0.15 0.15 0.5] Generamos las casas de manera aleatoria
  (for _index (range 0 (Variables|Default|GetNumberOfHouses))
    (Variables|Default|SetCandidateLocation (Math|Random|RandomPointinBoundingBox "0, 0, 0" (Variables|Default|GetMapSIze)))
    (Variables|Default|SetIsValidLocation true)
    (bind _array_element (Utilities|Array|ForEachLoopwithBreak (Variables|Default|GetOccupiedLocations) :!label _label)
      (:LoopBody
        (Variables|Default|SetIsValidLocation (< (Math|Vector|Distance(Vector) (Variables|Default|GetCandidateLocation) _array_element) 3e+01))
        (if (not (< (Math|Vector|Distance(Vector) (Variables|Default|GetCandidateLocation) _array_element) 3e+01))
          (goto _label Break)))
      (:Completed
        (Utilities|Array|Add (Variables|Default|GetOccupiedLocations) (Variables|Default|GetCandidateLocation))
        (bind _returnvalue (Game|SpawnActorfromClass "/Game/Background/BP_GenericHouse.BP_GenericHouse_C" (Math|Conversions|ToTransform(Vector) (Variables|Default|GetCandidateLocation)) "Undefined" "MultiplyWithRoot" 0 0))
        (Components|StaticMesh|SetStaticMesh (Variables|/Game/Background/BP_GenericHouse.BP_GenericHouse_C|GetStaticMesh _returnvalue) (.OutItem (Utilities|Array|Random (Variables|Default|GetHouseMeshed))))))))

(event Collision|EventActorBeginOverlap
  (params (OtherActor :type Actor%20Object%20Reference)))

(event EventTick
  (params (DeltaSeconds :type Float%20%28single-precision%29)))

(fn ConstructionScript)