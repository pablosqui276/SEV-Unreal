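; Enemy projectile actor that punishes the player on contact and can be reflected back at the archers.
; Overlapping BP_Player reloads BaseLevel; overlapping BP_Enemy_Archer after a return kills it, destroys the projectile and decrements the enemy count in GM_MyGameMode.
; ReturnProjectile flags it as returned, negates its ProjectileMovement velocity, faces it along the player's forward vector and refreshes its lifespan.
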(event Custom|ReturnProjectile
  (bind _projectilemovement (Variables|Default|GetProjectileMovement))
  (Variables|Default|SetisReturned true)
  (Variables|/Script/Engine.MovementComponent|SetVelocity _projectilemovement (Math|Vector|NegateVector (Variables|/Script/Engine.MovementComponent|GetVelocity _projectilemovement)))
  (Transformation|SetActorRotation (Math|Conversions|RotationFromXVector (Transformation|GetActorForwardVector (Game|GetPlayerCharacter 0))))
  (Actor|SetLifeSpan 6.0))

(event EventBeginPlay)

(event Collision|EventActorBeginOverlap
  (params (OtherActor :type Actor%20Object%20Reference))
  (Utilities|Casting|CastToBP_Player OtherActor
    (:then
      (Game|OpenLevel(byName) "BaseLevel"))
    (:CastFailed
      ;[0.15 0.15 0.15 0.5] Si golpea a otro enemyArcher
      (bind _asbp_enemy_archer (Utilities|Casting|CastToBP_Enemy_Archer OtherActor))
      (if (Variables|Default|GetisReturned)
        ;;[0.15 0.15 0.15 0.5] Si está activo el retorno
        (Default|Dead _asbp_enemy_archer)
        (Actor|DestroyActor)
        (bind _asgm_my_game_mode (Utilities|Casting|CastToGM_MyGameMode (Game|GetGameMode)))
        (Default|OneEnemyLess _asgm_my_game_mode)))))

(event EventTick
  (params (DeltaSeconds :type Float%20%28single-precision%29)))

(fn ConstructionScript)