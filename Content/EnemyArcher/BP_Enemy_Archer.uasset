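; Archer enemy character that fires projectiles at the player and updates its AI blackboard on death.
; Shoot briefly pauses movement around spawning BP_EnemyProjectile, behind a DoOnce with no reset.
; Dead, also gated once, stops movement, sets IsDead, plays an explosion and sound, and expires after a delay.
; Older timer-driven chase and patrol logic is disconnected and never runs.
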(event Custom|FollowPlayer
  ;[0.15 0.15 0.15 0.5] SI está a menos de 10 metros
)

(event Custom|Shoot
  (Utilities|FlowControl|DoOnce false
    (:Completed
      ;[0.15 0.15 0.15 0.5] Desactivar movimiento
      (Components|Activation|SetActive (Variables|Character|GetCharacterMovement) false false)
      (Utilities|FlowControl|Delay 0.2)
      (Game|SpawnActorfromClass "/Game/BP_EnemyProjectile.BP_EnemyProjectile_C" (Transformation|GetActorTransform) "Undefined" "MultiplyWithRoot" 0 0)
      (Utilities|FlowControl|Delay 0.2)
      (Components|Activation|SetActive (Variables|Character|GetCharacterMovement) true false))))

(event Custom|Dead
  (Utilities|FlowControl|DoOnce false
    (:Completed
      (Components|Activation|SetActive (Variables|Character|GetCharacterMovement) false false)
      (AI|Components|Blackboard|SetValueasBool (AI|GetBlackboard (AI|GetAIController self)) (Utilities|Name|MakeLiteralName "IsDead") true)
      (Actor|SetLifeSpan 5.0)
      ;[0.15 0.15 0.15 0.5] EXPLOSIÓN DIOS
      (Effects|SpawnEmitteratLocation "/Game/StarterContent/Particles/P_Explosion.P_Explosion" (Transformation|GetActorLocation))
      (Audio|PlaySound2D "/Game/Sounds/hit.hit" 1.0 1.0 0.0 0 0))))

(event EventBeginPlay)

(event Collision|EventActorBeginOverlap
  (params (OtherActor :type Actor%20Object%20Reference)))

(fn ConstructionScript)